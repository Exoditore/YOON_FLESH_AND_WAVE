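; Ranged enemy with directional sprites that chases a seen player, shoots projectiles and dies when its health runs out.
; A successful AI move near the player sets Bobba, letting Tick turn it toward them and fire impulse-launched projectiles on a delay.
; When Timer is negative, Attack also subtracts player health directly, with camera shake and sound.
; Death swaps every directional flipbook to Dead, disables collision and movement, then destroys the actor after a delay.
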(event OnSeePawn(PawnSensing)
  (params (Pawn :type Pawn%20Object%20Reference))
  ;[1 1 1] Cuando se ve Jugador
  (bind _asfirst_person_character (Utilities|Casting|CastToFirstPersonCharacter Pawn))
  (AI|AIMoveTo self "0, 0, 0" _asfirst_person_character 1.5e+03 false
    (:OnSuccess
      (Utilities|FlowControl|DoOnce false :!label _label
        (:Completed
          (Variables|Default|Setbobba true))))
    (:OnFail
      (Variables|Default|Setbobba false)
      (goto _label Reset))))

(event Custom|wow
  (if (and (Variables|Default|Getbobba) (not (Variables|Default|Getded)))
    (Utilities|FlowControl|Sequence
      (:then_0
        (bind _asfirst_person_character (Utilities|Casting|CastToFirstPersonCharacter (Game|GetPlayerCharacter 0)))
        (Transformation|SetActorRotation (Math|Rotator|FindLookatRotation (Transformation|GetActorLocation) (Transformation|GetActorLocation _asfirst_person_character))))
      (:then_1
        (if (Variables|Default|GetSpawnProjectile)
          (bind _returnvalue (Game|SpawnActorfromClass "/Game/FirstPersonBP/Blueprints/FirstPersonProjectile.FirstPersonProjectile_C" (Transformation|GetWorldTransform (Variables|Default|GetShoot)) "Undefined" 0 0))
          (Physics|AddImpulse (Variables|/Game/FirstPersonBP/Blueprints/FirstPersonProjectile.FirstPersonProjectile_C|GetCollisionComponent _returnvalue) (* (Math|Vector|GetForwardVector (Variables|Default|GetShoot)) (Variables|Default|GetImpulse)) "None" false)
          (Variables|Default|SetSpawnProjectile false)
          (Utilities|FlowControl|Delay 0.5)
          (Variables|Default|SetSpawnProjectile true))))))

(event Custom|Attack
  ;[1 1 1] Atacar
  (if (and (Variables|Default|GetCanAttack) (not false))
    (Variables|Default|SetCanAttack false)
    (Class|MatineeCameraShake|StartMatineeCameraShake (Game|GetPlayerCameraManager 0) "/Game/Shake/PlayerDamage.PlayerDamage_C" 1.0 "CameraLocal" "0, 0, 0")
    (bind _asfirst_person_character (Utilities|Casting|CastToFirstPersonCharacter (Game|GetPlayerCharacter 0)))
    (Audio|PlaySound2D "/Game/SFX/Damage/Damage.Damage" 1.0 1.0 0.0 0 0)
    (bind _output_get (Variables|/Game/FirstPersonBP/Blueprints/FirstPersonCharacter.FirstPersonCharacter_C|SetHealth _asfirst_person_character (- (Variables|/Game/FirstPersonBP/Blueprints/FirstPersonCharacter.FirstPersonCharacter_C|GetHealth _asfirst_person_character) 3e+01)))
    (Development|PrintString (Utilities|String|ToString(Float) _output_get) true true "(R=1.000000,G=0.068094,B=0.000000,A=1.000000)")
    (Utilities|FlowControl|Delay 0.5)
    (Variables|Default|SetCanAttack true)))

(event EventTick
  (params (DeltaSeconds :type Float%20%28single-precision%29))
  ;[1 1 1] Tik tak toe
  (|CallParentFunction 0.0)
  (CallFunction|Wow)
  (if (and (Variables|Default|Getbobba) (< (Variables|Default|GetTimer) 0.0))
    (CallFunction|Attack)))

(event Collision|EventActorBeginOverlap
  (params (OtherActor :type Actor%20Object%20Reference))
  (|CallParentFunction OtherActor) ; This node is disabled and will not be called.\nDrag off pins to build functionality.
)

(event Game|Damage|EventAnyDamage
  (params (Damage :type Float%20%28single-precision%29) (DamageType :type Damage%20Type%20Object%20Reference) (InstigatedBy :type Controller%20Object%20Reference) (DamageCauser :type Actor%20Object%20Reference))
  ;[1 1 1] ded
  (Variables|Default|SetVida (- (Variables|Default|GetVida) Damage))
  (if (<= (Variables|Default|GetVida) 0.0)
    (Variables|Default|Setded true)
    (Utilities|FlowControl|DoOnce false
      (:Completed
        (Variables|Default|Setbobba false)
        (Audio|PlaySoundatLocation "/Game/SFX/Damage/ayylamao.ayylamao" (Transformation|GetWorldLocation (Variables|Character|GetMesh)) "0, 0, 0" 1.0 1.0 0.0 0 0 0)
        (Transformation|SetRelativeLocation (Variables|Default|GetPaperFlipbook) (Variables|/Script/Engine.SceneComponent|GetRelativeLocation (Variables|Default|GetPaperSprite)) false false)
        (Variables|Default|SetFront "/Game/Textures/Monster/Dead.Dead")
        (Variables|Default|SetLeftBack "/Game/Textures/Monster/Dead.Dead")
        (Variables|Default|SetBack "/Game/Textures/Monster/Dead.Dead")
        (Variables|Default|SetFrontLeft "/Game/Textures/Monster/Dead.Dead")
        (Variables|Default|SetRightBack "/Game/Textures/Monster/Dead.Dead")
        (Variables|Default|SetRightFront "/Game/Textures/Monster/Dead.Dead")
        (Variables|/Script/Engine.CharacterMovementComponent|SetMaxWalkSpeed (Variables|Character|GetCharacterMovement) 0.0)
        (Collision|SetCollisionEnabled (Variables|Default|GetCapsuleComponent) "NoCollision")
        (Variables|Default|SetDead? true)
        (Utilities|FlowControl|Delay 4.9)
        (Actor|DestroyActor)))
    (else
      (Audio|PlaySound2D "/Game/SFX/Damage/enemyHIT.enemyHIT" 1.0 1.0 0.0 0 0))))

(event EventBeginPlay
  ;[1 1 1] si
  (|CallParentFunction))

(fn ConstructionScript
  (|CallParentFunction))

(fn AiMove)