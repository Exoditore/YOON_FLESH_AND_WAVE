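; BP_TipaxD is a melee enemy with directional Paper2D flipbooks that chases and damages the player.
; PawnSensing starts AI MoveTo; reaching the player plus box overlap runs a per-tick countdown before attacking.
; Attacks subtract player Health directly, repeating on a short delay-based cooldown.
; The ded event swaps all directional art to Dead, stops movement and collision, then destroys the actor after a delay.
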(event OnSeePawn(PawnSensing)
  (params (Pawn :type Pawn%20Object%20Reference))
  ;[1 1 1] Cuando se ve Jugador
  (bind _asfirst_person_character (Utilities|Casting|CastToFirstPersonCharacter Pawn))
  (AI|AIMoveTo self "0, 0, 0" _asfirst_person_character 1e+02 false
    (:OnSuccess
      (Utilities|FlowControl|DoOnce false :!label _label
        (:Completed
          (Variables|Default|Setbobba true))))
    (:OnFail
      (Variables|Default|Setbobba false)
      (goto _label Reset))))

(event OnComponentBeginOverlap(Box)
  (params (OverlappedComponent :type Primitive%20Component%20Object%20Reference) (OtherActor :type Actor%20Object%20Reference) (OtherComp :type Primitive%20Component%20Object%20Reference) (OtherBodyIndex :type Integer) (bFromSweep :type Boolean) (SweepResult :type Hit%20Result%20Structure%20%28by%20ref%29))
  ;[1 1 1] Collision (Apply Damage)
  (Utilities|Casting|CastToFirstPersonCharacter OtherActor)
  (Variables|Default|Setiscol true))

(event OnComponentEndOverlap(Box)
  (params (OverlappedComponent :type Primitive%20Component%20Object%20Reference) (OtherActor :type Actor%20Object%20Reference) (OtherComp :type Primitive%20Component%20Object%20Reference) (OtherBodyIndex :type Integer))
  ;[1 1 1] Collision (Apply Damage)
  (Utilities|Casting|CastToFirstPersonCharacter OtherActor)
  (Variables|Default|Setiscol false))

(event Custom|Attack
  ;[1 1 1] Atacar
  (if (and (Variables|Default|GetCanAttack) (not false))
    (Variables|Default|SetCanAttack false)
    (bind _asfirst_person_character (Utilities|Casting|CastToFirstPersonCharacter (Game|GetPlayerCharacter 0)))
    (Audio|PlaySound2D "/Game/SFX/Damage/Damage.Damage" 1.0 1.0 0.0 0 0)
    (bind _output_get (Variables|/Game/FirstPersonBP/Blueprints/FirstPersonCharacter.FirstPersonCharacter_C|SetHealth _asfirst_person_character (- (Variables|/Game/FirstPersonBP/Blueprints/FirstPersonCharacter.FirstPersonCharacter_C|GetHealth _asfirst_person_character) 3e+01)))
    (Development|PrintString (Utilities|String|ToString(Float) _output_get) true true "(R=1.000000,G=0.068094,B=0.000000,A=1.000000)")
    (Utilities|FlowControl|Delay 0.5)
    (Variables|Default|SetCanAttack true)))

(event Custom|yee
  ;[1 1 1] Timer En colision
  (if (and (Variables|Default|Getbobba) (Variables|Default|Getiscol))
    (Variables|Default|SetTimer (- (Variables|Default|GetTimer) 1.0))
    (else
      (Variables|Default|SetTimer 1e+01))))

(event Custom|ded
  ;[1 1 1] ded
  (Utilities|FlowControl|DoOnce false
    (:Completed
      (Audio|PlaySoundatLocation "/Game/SFX/Damage/ayylamao.ayylamao" (Transformation|GetWorldLocation (Variables|Character|GetMesh)) "0, 0, 0" 1.0 1.0 0.0 0 0 0)
      (Transformation|SetRelativeLocation (Variables|Default|GetPaperFlipbook) (Variables|/Script/Engine.SceneComponent|GetRelativeLocation (Variables|Default|GetPaperSprite)) false false)
      (Variables|Default|SetFront "/Game/Textures/Monster/Dead.Dead")
      (Variables|Default|SetLeftBack "/Game/Textures/Monster/Dead.Dead")
      (Variables|Default|SetBack "/Game/Textures/Monster/Dead.Dead")
      (Variables|Default|SetFrontLeft "/Game/Textures/Monster/Dead.Dead")
      (Variables|Default|SetRightBack "/Game/Textures/Monster/Dead.Dead")
      (Variables|Default|SetRightFront "/Game/Textures/Monster/Dead.Dead")
      (Variables|/Script/Engine.CharacterMovementComponent|SetMaxWalkSpeed (Variables|Character|GetCharacterMovement) 0.0)
      (Collision|SetCollisionEnabled (Variables|Default|GetCapsuleComponent) "NoCollision")
      (Variables|Default|SetDead? true)
      (Collision|SetCollisionEnabled (Variables|Default|GetBox) "NoCollision")
      (Utilities|FlowControl|Delay 4.9)
      (Actor|DestroyActor))))

(event EventTick
  (params (DeltaSeconds :type Float%20%28single-precision%29))
  ;[1 1 1] Tik tak toe
  (|CallParentFunction 0.0)
  (CallFunction|Yee)
  (if (and (Variables|Default|Getbobba) (< (Variables|Default|GetTimer) 0.0))
    (CallFunction|Attack)))

(event Collision|EventActorBeginOverlap
  (params (OtherActor :type Actor%20Object%20Reference))
  (|CallParentFunction OtherActor) ; This node is disabled and will not be called.\nDrag off pins to build functionality.
)

(event EventBeginPlay
  ;[1 1 1] si
  (|CallParentFunction))

(fn ConstructionScript
  (|CallParentFunction))

(fn AiMove)